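; BP_MovingLight is an example actor that moves a point light and a sphere component along a circular path.
; Tick accumulates time and builds an XY vector from its cosine and sine, using RotationSpeed and RotationScale, with no Z movement.
; That vector is added as a local offset to both components every frame, so it acts as a per-frame step and the path depends on frame rate.
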(event EventBeginPlay)

(event Collision|EventActorBeginOverlap
  (params (OtherActor :type Actor%20Object%20Reference)))

(event EventTick
  (params (DeltaSeconds :type Float%20%28single-precision%29))
  (bind _rotationscale (Variables|Default|GetRotationScale))
  (bind _output_get (Variables|Default|SetTime (+ DeltaSeconds (Variables|Default|GetTime))))
  (Transformation|AddLocalOffset (Variables|Default|GetPointLight) (+ "" (Math|Vector|MakeVector (* (Math|Trig|Cos(Radians) (* (Variables|Default|GetRotationSpeed) _output_get)) _rotationscale) (* (Math|Trig|Sin(Radians) (* (Variables|Default|GetRotationSpeed) _output_get)) _rotationscale) 0.0)) false false)
  (Transformation|AddLocalOffset (Variables|Default|GetSphere) (+ "" (Math|Vector|MakeVector (* (Math|Trig|Cos(Radians) (* (Variables|Default|GetRotationSpeed) _output_get)) _rotationscale) (* (Math|Trig|Sin(Radians) (* (Variables|Default|GetRotationSpeed) _output_get)) _rotationscale) 0.0)) false false))

(fn ConstructionScript)